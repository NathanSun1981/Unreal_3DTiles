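; Satellite actor that tracks whether it lies within the player's field of view.
; Each Tick, it takes the angle between the pawn-to-satellite direction and the player controller's forward vector, and sets IsVisible when that is within half the camera FOV.
; The test is a pure angular cone with no occlusion check.
; Freelook input, BeginPlay and overlap events are empty; disconnected debug and rotation nodes remain unused.
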(event `self.ReceiveBeginPlay`)

(event `self.ReceiveActorBeginOverlap`
  (params (OtherActor :type "Actor Object Reference")))

(event `self.ReceiveTick`
  (params (DeltaSeconds :type "Float (single-precision)"))
  ;[1 1 1] check if satellite is in fov
  (if (<= (`KismetMathLibrary.DegAcos` (`KismetMathLibrary.Dot_VectorVector` (`KismetMathLibrary.Normal` (- (`self.K2_GetActorLocation`) (`self.K2_GetActorLocation` (`GameplayStatics.GetPlayerPawn` 0)))) (`self.GetActorForwardVector` (`GameplayStatics.GetPlayerController` 0)))) (/ (`PlayerCameraManager.GetFOVAngle` (`GameplayStatics.GetPlayerCameraManager` 0)) 2.0))
    (set `self.isVisible` true)
    (else
      (set `self.isVisible` false))))

(event `InputAxis|FreelookHori`
  (params (AxisValue :type "Float (single-precision)"))
  ;[1 1 1] SpringArm Rotation
)

(event `InputAxis|FreelookVec`
  (params (AxisValue :type "Float (single-precision)"))
  ;[1 1 1] SpringArm Rotation
)

(event `Key|LeftMouseButton`
  (params (Key :type "Key Structure")))

(fn `UserConstructionScript`)